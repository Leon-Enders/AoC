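; Fire Monk gameplay ability Rising Kick of the Flame, which plays a dash-style kick montage aimed at a target location.
; A TargetDataForDash task supplies the destination, which the avatar receives as a warp target through CombatInterface before the montage starts.
; The ability ends when the montage completes or is cancelled, or after a short delay if it is interrupted.
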(event `self.K2_ActivateAbility`
  (bind (_asynctaskproxy _datahandle) (`TargetDataForDash.CreateTargetDataForDash` 400.0)
    (:`ValidData`
      (bind _ascombat_interface (cast `CombatInterface` (`self.GetAvatarActorFromActorInfo`)))
      (bind _returnvalue_location (`KismetMathLibrary.BreakTransform` (`AbilitySystemBlueprintLibrary.GetTargetDataEndPointTransform` _datahandle)))
      (set `self.DashTargetLocation` _returnvalue_location)
      (message `CombatInterface.SetWarpTarget` (`KismetSystemLibrary.Conv_InterfaceToObject` _ascombat_interface) (`self.DashTargetLocation`))
      (`AbilityTask_PlayMontageAndWait.CreatePlayMontageAndWaitProxy` "None" "/Game/Assets/Characters/FireMonk/Animations/Abilities/AM_FireMonk_RisingKickOfTheFlame.AM_FireMonk_RisingKickOfTheFlame"
        (:`OnCompleted`
          _)
        (:`OnInterrupted`
          (`KismetSystemLibrary.Delay` 0.1))
        (:`OnCancelled`
          _))
      (`self.K2_EndAbility`))))