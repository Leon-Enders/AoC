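; Gameplay ability for the Fire Monk's flying kick, a targeted dash driven by an animation montage.
; A TargetDataForDash task supplies an end point, which the avatar receives as a warp target through CombatInterface.
; The flying kick montage then plays, and the ability ends on completion or cancellation, or after a brief delay when interrupted.
; A TODO notes planned input flags to disable directions.
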(event `self.K2_ActivateAbility`
  ;[1 1 1] TODO: Create Input Flags to disable directions
  (bind (_asynctaskproxy _datahandle) (`TargetDataForDash.CreateTargetDataForDash` 1000.0)
    (:`ValidData`
      (bind _ascombat_interface (cast `CombatInterface` (`self.GetAvatarActorFromActorInfo`)))
      (bind _returnvalue_location (`KismetMathLibrary.BreakTransform` (`AbilitySystemBlueprintLibrary.GetTargetDataEndPointTransform` _datahandle)))
      (set `self.DashTargetLocation` _returnvalue_location)
      (message `CombatInterface.SetWarpTarget` (`KismetSystemLibrary.Conv_InterfaceToObject` _ascombat_interface) (`self.DashTargetLocation`))
      (`AbilityTask_PlayMontageAndWait.CreatePlayMontageAndWaitProxy` "None" "/Game/Assets/Characters/FireMonk/Animations/Abilities/AM_FireMonk_FlyingKick.AM_FireMonk_FlyingKick"
        (:`OnCompleted`
          _)
        (:`OnInterrupted`
          (`KismetSystemLibrary.Delay` 0.1))
        (:`OnCancelled`
          _))
      (`self.K2_EndAbility`))))