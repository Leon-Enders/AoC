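; Fire Monk gameplay ability that spawns BP_LaunchExplosion and launches the avatar character.
; A TargetDataForLaunch task supplies the explosion's origin, the movement direction and the launch velocity, which is packed as the target data's end-point location.
; Forward/back input takes priority over left/right when choosing the montage section, with Idle as fallback.
; The ability ends after a short delay once the montage completes or is interrupted.
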(event `self.K2_ActivateAbility`
  (bind (_asynctaskproxy _datahandle _lrdirection _fwdirection) (`TargetDataForCharacterLaunch.CreateTargetDataForLaunch` 3.0)
    (:`ValidData`
      (set `self.LaunchVelocity` (.location (`AbilitySystemBlueprintLibrary.GetTargetDataEndPointTransform` _datahandle)))
      (bind _ascharacter (cast `Character` (`self.GetAvatarActorFromActorInfo`)))
      (`GameplayTask_SpawnActor.SpawnActor` null (.location (`AbilitySystemBlueprintLibrary.GetTargetDataOrigin` _datahandle)) (struct) "/Game/Blueprints/Abilitysystem/GameplayAbilities/FireMonk/LaunchExplosion/BP_LaunchExplosion.BP_LaunchExplosion_C" false null
        (:`then`
          (`Character.LaunchCharacter` _ascharacter (`self.LaunchVelocity`) true true)
          (switch `EInputDirection` _fwdirection
            (:`E_Forward`
              (switch `EInputDirection` _lrdirection
                (:`E_Left`
                  _)
                (:`E_Right`
                  _)
                (:`E_None`
                  _))
              (`AbilityTask_PlayMontageAndWait.CreatePlayMontageAndWaitProxy` "None" "/Game/Assets/Characters/FireMonk/Animations/Abilities/LaunchExplosion/AM_LaunchExplosion.AM_LaunchExplosion" 1.0 "Forward"
                (:`OnCompleted`
                  _)
                (:`OnInterrupted`
                  _)))
            (:`E_Back`
              (switch `EInputDirection` _lrdirection
                (:`E_Left`
                  _)
                (:`E_Right`
                  _)
                (:`E_None`
                  _))
              (`AbilityTask_PlayMontageAndWait.CreatePlayMontageAndWaitProxy` "None" "/Game/Assets/Characters/FireMonk/Animations/Abilities/LaunchExplosion/AM_LaunchExplosion.AM_LaunchExplosion" 1.0 "Backward"
                (:`OnCompleted`
                  _)
                (:`OnInterrupted`
                  _)))
            (:`E_None`
              (switch `EInputDirection` _lrdirection
                (:`E_Left`
                  (`AbilityTask_PlayMontageAndWait.CreatePlayMontageAndWaitProxy` "None" "/Game/Assets/Characters/FireMonk/Animations/Abilities/LaunchExplosion/AM_LaunchExplosion.AM_LaunchExplosion" 1.0 "Left"
                    (:`OnCompleted`
                      _)
                    (:`OnBlendOut`
                      _)
                    (:`OnInterrupted`
                      _)
                    (:`OnCancelled`
                      _)))
                (:`E_Right`
                  (`AbilityTask_PlayMontageAndWait.CreatePlayMontageAndWaitProxy` "None" "/Game/Assets/Characters/FireMonk/Animations/Abilities/LaunchExplosion/AM_LaunchExplosion.AM_LaunchExplosion" 1.0 "Right"
                    (:`OnCompleted`
                      _)
                    (:`OnInterrupted`
                      _)))
                (:`E_None`
                  (`AbilityTask_PlayMontageAndWait.CreatePlayMontageAndWaitProxy` "None" "/Game/Assets/Characters/FireMonk/Animations/Abilities/LaunchExplosion/AM_LaunchExplosion.AM_LaunchExplosion" 1.0 "Idle"
                    (:`OnCompleted`
                      _)
                    (:`OnInterrupted`
                      _))))))
          (`KismetSystemLibrary.Delay` 3.0)
          (`self.K2_EndAbility`))))))