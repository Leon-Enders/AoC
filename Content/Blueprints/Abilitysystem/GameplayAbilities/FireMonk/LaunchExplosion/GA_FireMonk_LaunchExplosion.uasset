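; Fire Monk Launch Explosion gameplay ability that launches the avatar character and plays its launch montage.
; A TargetDataForLaunch task supplies the velocity through the target data's end point, which overrides the character's current velocity.
; The montage always starts at its "Left" section, as the switch choosing sections by movement direction is disconnected.
; The ability ends after a short delay once the montage finishes or is interrupted.
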(event `self.K2_ActivateAbility`
  (bind (_asynctaskproxy _datahandle _lrdirection _fwdirection) (`TargetDataForCharacterLaunch.CreateTargetDataForLaunch` 3.0)
    (:`ValidData`
      (set `self.LaunchVelocity` (.location (`AbilitySystemBlueprintLibrary.GetTargetDataEndPointTransform` _datahandle)))
      (bind _ascharacter (cast `Character` (`self.GetAvatarActorFromActorInfo`)))
      (`Character.LaunchCharacter` _ascharacter (`self.LaunchVelocity`) true true)
      (`AbilityTask_PlayMontageAndWait.CreatePlayMontageAndWaitProxy` "None" "/Game/Assets/Characters/FireMonk/Animations/Abilities/LaunchExplosion/AM_FireMonk_LaunchExplosion.AM_FireMonk_LaunchExplosion" 1.0 "Left"
        (:`OnCompleted`
          _)
        (:`OnBlendOut`
          _)
        (:`OnInterrupted`
          _)
        (:`OnCancelled`
          _))
      (`KismetSystemLibrary.Delay` 3.0)
      (`self.K2_EndAbility`))))