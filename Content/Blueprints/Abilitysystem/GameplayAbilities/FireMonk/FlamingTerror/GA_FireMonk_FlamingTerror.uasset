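; Fire Monk Flaming Terror gameplay ability that fires a rapid volley of fireballs toward the crosshair during a montage.
; A repeat action spawns eight projectiles at short intervals, with a FlipFlop alternating the AB flag passed to each.
; Meanwhile, a delayed loop keeps refreshing the target from crosshair data, using the hit location or trace end point.
; The ability ends shortly after the montage completes, blends out or is interrupted.
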(event `self.K2_ActivateAbility`
  (bind (_asynctaskproxy _datahandle _bhit) (`TargetDataUnderCrosshair.CreateTargetDataUnderCrosshair`)
    (:`ValidData`
      (if _bhit
        (set `self.TargetLocation` (`.Location` (`GameplayStatics.BreakHitResult` (`AbilitySystemBlueprintLibrary.GetHitResultFromTargetData` _datahandle))))
        (else
          (bind _returnvalue_location (`KismetMathLibrary.BreakTransform` (`AbilitySystemBlueprintLibrary.GetTargetDataEndPointTransform` _datahandle)))
          (set `self.TargetLocation` _returnvalue_location)))
      (`AbilityTask_PlayMontageAndWait.CreatePlayMontageAndWaitProxy` "None" "/Game/Assets/Characters/FireMonk/Animations/Abilities/AM_FireMonk_FlamingTerror.AM_FireMonk_FlamingTerror"
        (:`then`
          ;[1 1 1] Get NewTarget Data for each Fireball
          (`AbilityTask_Repeat.RepeatAction` 0.15 8
            (:`then`
              (bind (_asynctaskproxy_2 _datahandle_2 _bhit_2) (`TargetDataUnderCrosshair.CreateTargetDataUnderCrosshair` :!label _label)
                (:`ValidData`
                  (if _bhit_2
                    (set `self.TargetLocation` (`.Location` (`GameplayStatics.BreakHitResult` (`AbilitySystemBlueprintLibrary.GetHitResultFromTargetData` _datahandle_2))))
                    (`KismetSystemLibrary.Delay` 0.1)
                    (goto _label)
                    (else
                      (bind _returnvalue_location_2 (`KismetMathLibrary.BreakTransform` (`AbilitySystemBlueprintLibrary.GetTargetDataEndPointTransform` _datahandle_2)))
                      (set `self.TargetLocation` _returnvalue_location_2)
                      (`KismetSystemLibrary.Delay` 0.1)
                      (goto _label))))))
            (:`OnPerformAction`
              (bind _isa (`/Engine/EditorBlueprintResources/StandardMacros.FlipFlop`)
                (:`A`
                  _)
                (:`B`
                  _))
              (`self.SpawnProjectile` (`self.TargetLocation`) _isa))))
        (:`OnCompleted`
          (`KismetSystemLibrary.Delay` 1.0 :!label _label_2)
          (`self.K2_EndAbility`))
        (:`OnBlendOut`
          (goto _label_2))
        (:`OnInterrupted`
          (goto _label_2))
        (:`OnCancelled`
          (goto _label_2))))))

(event `self.K2_OnEndAbility`
  (params (bWasCancelled :type Boolean)))