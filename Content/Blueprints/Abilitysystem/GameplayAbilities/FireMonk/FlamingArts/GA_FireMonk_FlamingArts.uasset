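; Fire Monk Flaming Arts dash ability that applies a gameplay effect to its owner, intended to block other abilities while dashing.
; A custom target-data task supplies an endpoint, passed through CombatInterface as the warp target, and a tag naming the montage start section.
; The effect is removed on the montage event, blend out or cancel.
; The ability ends on interruption or two seconds after montage completion.
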(event `self.K2_ActivateAbility`
  ;[1 1 1] Apply GameplayTag to block other abilities while dashing
  (bind _returnvalue (`self.BP_ApplyGameplayEffectToOwner` "/Game/Blueprints/Abilitysystem/GameplayEffects/Effects/FireMonk/GE_FireMonk_FlamingArts.GE_FireMonk_FlamingArts_C"))
  (set `self.ActiveGameplayEffectHandle` _returnvalue)
  (bind (_asynctaskproxy _datahandle _activationtag) (`TargetDataForDash.CreateTargetDataForDash` (`self.DashDistance`))
    (:`ValidData`
      (set `self.AnimationTagName` (`BlueprintGameplayTagLibrary.GetTagName` _activationtag))
      (bind _ascombat_interface (cast `CombatInterface` (`self.GetAvatarActorFromActorInfo`)))
      (bind _returnvalue_location (`KismetMathLibrary.BreakTransform` (`AbilitySystemBlueprintLibrary.GetTargetDataEndPointTransform` _datahandle)))
      (set `self.DashTargetLocation` _returnvalue_location)
      (message `CombatInterface.SetWarpTarget` (`KismetSystemLibrary.Conv_InterfaceToObject` _ascombat_interface) (`self.DashTargetLocation`))
      (`AbilityTask_PlayMontageAndWait.CreatePlayMontageAndWaitProxy` "None" "/Game/Assets/Characters/FireMonk/Animations/Abilities/FlamingArts/AM_FireMonk_FlamingArts_Forward.AM_FireMonk_FlamingArts_Forward" 1.0 (`self.AnimationTagName`)
        (:`then`
          (`AbilityTask_WaitGameplayEvent.WaitGameplayEvent` (struct :`TagName` "Event.Montage.FlamingArts") null true
            (:`EventReceived`
              (`KismetSystemLibrary.PrintString` "Dash Event")
              (`self.BP_RemoveGameplayEffectFromOwnerWithHandle` (`self.ActiveGameplayEffectHandle`)))))
        (:`OnCompleted`
          (`KismetSystemLibrary.PrintString` "On Completed")
          (`KismetSystemLibrary.Delay` 2.0)
          (`self.K2_EndAbility` :!label _label))
        (:`OnBlendOut`
          (`KismetSystemLibrary.PrintString` "Oh Blended")
          (`self.BP_RemoveGameplayEffectFromOwnerWithHandle` (`self.ActiveGameplayEffectHandle`) :!label _label_2)
          (`AbilityTask_NetworkSyncPoint.WaitNetSync` "BothWait"))
        (:`OnInterrupted`
          (`KismetSystemLibrary.PrintString` "On Interrupted")
          (goto _label))
        (:`OnCancelled`
          (goto _label_2))))))