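; Gameplay ability for the Fire Monk's Flaming Arts, a dash attack or move driven by a montage.
; A custom TargetDataForDash task supplies the end point and an activation tag from the dash distance.
; The end point goes to the avatar through CombatInterface as a warp target, and the tag name selects the montage's start section.
; The ability ends when the montage completes, blends out, is interrupted or is cancelled.
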(event `self.K2_ActivateAbility`
  (bind (_asynctaskproxy _datahandle _activationtag) (`TargetDataForDash.CreateTargetDataForDash` (`self.DashDistance`))
    (:`ValidData`
      (set `self.AnimationTagName` (`BlueprintGameplayTagLibrary.GetTagName` _activationtag))
      (bind _ascombat_interface (cast `CombatInterface` (`self.GetAvatarActorFromActorInfo`)))
      (bind _returnvalue_location (`KismetMathLibrary.BreakTransform` (`AbilitySystemBlueprintLibrary.GetTargetDataEndPointTransform` _datahandle)))
      (set `self.DashTargetLocation` _returnvalue_location)
      (message `CombatInterface.SetWarpTarget` (`KismetSystemLibrary.Conv_InterfaceToObject` _ascombat_interface) (`self.DashTargetLocation`))
      (`AbilityTask_PlayMontageAndWait.CreatePlayMontageAndWaitProxy` "None" "/Game/Assets/Characters/FireMonk/Animations/Abilities/FlamingArts/AM_FireMonk_FlamingArts_Forward.AM_FireMonk_FlamingArts_Forward" 1.0 (`self.AnimationTagName`)
        (:`OnCompleted`
          _)
        (:`OnBlendOut`
          _)
        (:`OnInterrupted`
          _)
        (:`OnCancelled`
          _))
      (`self.K2_EndAbility`))))