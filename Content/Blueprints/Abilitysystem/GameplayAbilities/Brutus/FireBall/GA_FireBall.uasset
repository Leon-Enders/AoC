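; Brutus's fireball gameplay ability, which casts a projectile toward the point under the crosshair.
; On activation, a crosshair target data task supplies the target location: the blocking hit point, or the target data's end point when nothing blocks.
; It plays the cast montage and waits for the fireball montage gameplay event on the avatar to call SpawnProjectile.
; The ability ends after a short delay following the spawn.
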(event `self.K2_ActivateAbility`
  (bind (_asynctaskproxy _datahandle) (`TargetDataUnderCrosshair.CreateTargetDataUnderCrosshair`)
    (:`ValidData`
      (bind (_bblockinghit _binitialoverlap _time _distance _location) (`GameplayStatics.BreakHitResult` (`AbilitySystemBlueprintLibrary.GetHitResultFromTargetData` _datahandle)))
      (if _bblockinghit
        (set `self.TargetLocation` _location)
        (else
          (bind _returnvalue_location (`KismetMathLibrary.BreakTransform` (`AbilitySystemBlueprintLibrary.GetTargetDataEndPointTransform` _datahandle)))
          (set `self.TargetLocation` _returnvalue_location)))
      (`AbilityTask_PlayMontageAndWait.CreatePlayMontageAndWaitProxy` "None" "/Game/Assets/Characters/StylizedCharacter/Animations/AM_Cast.AM_Cast"
        (:`then`
          (`AbilityAsync_WaitGameplayEvent.WaitGameplayEventToActor` (`self.GetAvatarActorFromActorInfo`) (struct :`TagName` "Event.Montage.Fireball")
            (:`EventReceived`
              (`self.SpawnProjectile` (`self.TargetLocation`))
              (`KismetSystemLibrary.Delay` 0.5)
              (`self.K2_EndAbility`))))))))

(event `self.K2_OnEndAbility`
  (params (bWasCancelled :type Boolean)))