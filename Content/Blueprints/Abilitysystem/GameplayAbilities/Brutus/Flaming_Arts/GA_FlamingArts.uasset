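; Brutus's Flaming Arts gameplay ability, a left or right dodge dash to a targeted location.
; A target-data task, given the dash distance, supplies the destination and side, then a particle spawns at that point.
; The destination is passed through the avatar's CombatInterface as a warp target before the matching dodge montage plays.
; The ability ends shortly after montage blend-out, or immediately on interruption.
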(event `self.K2_ActivateAbility`
  (bind (_asynctaskproxy _datahandle _bisleft) (`TargetDataForDash.CreateTargetDataForDash` (`self.DashDistance`))
    (:`ValidData`
      (bind _ascombat_interface (cast `CombatInterface` (`self.GetAvatarActorFromActorInfo`)))
      (bind _returnvalue_location (`KismetMathLibrary.BreakTransform` (`AbilitySystemBlueprintLibrary.GetTargetDataEndPointTransform` _datahandle)))
      (set `self.DashTargetLocation` _returnvalue_location)
      (message `CombatInterface.SetWarpTarget` (`KismetSystemLibrary.Conv_InterfaceToObject` _ascombat_interface) (`self.DashTargetLocation`))
      (`self.SpawnParticle` (`self.DashTargetLocation`))
      (if _bisleft
        (`AbilityTask_PlayMontageAndWait.CreatePlayMontageAndWaitProxy` "None" "/Game/Assets/Characters/StylizedCharacter/Animations/AM_Dodge_Left.AM_Dodge_Left"
          (:`OnBlendOut`
            (`KismetSystemLibrary.Delay` 0.2)
            (`self.K2_EndAbility`))
          (:`OnInterrupted`
            (`self.K2_EndAbility`)))
        (else
          (`AbilityTask_PlayMontageAndWait.CreatePlayMontageAndWaitProxy` "None" "/Game/Assets/Characters/StylizedCharacter/Animations/AM_Dodge_Right.AM_Dodge_Right"
            (:`OnBlendOut`
              (`KismetSystemLibrary.Delay` 0.2)
              (`self.K2_EndAbility`))
            (:`OnInterrupted`
              (`self.K2_EndAbility`))))))))