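; BP_FireMonk is the Fire Monk champion character, built from modular mesh parts for body, armor and facial pieces.
; On BeginPlay, each part takes the main Mesh as its leader pose component so all pieces animate together.
; A SetWarpTarget event writes a given location into the Motion Warping "DashTarget", letting warped animations aim at that point.
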(event `CombatInterface.SetWarpTarget`
  (params (Location :type "Vector Structure (by ref)"))
  (`MotionWarpingComponent.AddOrUpdateWarpTargetFromLocation` (`self.MotionWarping`) "DashTarget" Location))

(event `self.ReceiveBeginPlay`
  ;[1 1 1] SetUp Character Model
  (`SkinnedMeshComponent.SetLeaderPoseComponent` (`self.Ears`) (`self.Mesh`) false false)
  (`SkinnedMeshComponent.SetLeaderPoseComponent` (`self.Facials_01`) (`self.Mesh`) false false)
  (`SkinnedMeshComponent.SetLeaderPoseComponent` (`self.Helmet`) (`self.Mesh`) false false)
  (`SkinnedMeshComponent.SetLeaderPoseComponent` (`self.Legs`) (`self.Mesh`) false false)
  (`SkinnedMeshComponent.SetLeaderPoseComponent` (`self.Hands`) (`self.Mesh`) false false)
  (`SkinnedMeshComponent.SetLeaderPoseComponent` (`self.HandsAdd`) (`self.Mesh`) false false)
  (`SkinnedMeshComponent.SetLeaderPoseComponent` (`self.Chest`) (`self.Mesh`) false false)
  (`SkinnedMeshComponent.SetLeaderPoseComponent` (`self.Bracers`) (`self.Mesh`) false false)
  (`SkinnedMeshComponent.SetLeaderPoseComponent` (`self.Boots`) (`self.Mesh`) false false)
  (`SkinnedMeshComponent.SetLeaderPoseComponent` (`self.Belt`) (`self.Mesh`) false false)
  (`SkinnedMeshComponent.SetLeaderPoseComponent` (`self.LegsAdd`) (`self.Mesh`) false false)
  (`SkinnedMeshComponent.SetLeaderPoseComponent` (`self.BracersAdd`) (`self.Mesh`) false false)
  (`SkinnedMeshComponent.SetLeaderPoseComponent` (`self.Shoulders`) (`self.Mesh`) false false))

(fn `UserConstructionScript`)