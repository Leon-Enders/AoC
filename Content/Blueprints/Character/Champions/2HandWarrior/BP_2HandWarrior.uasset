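; BP_2HandWarrior is the character Blueprint for the two-handed warrior champion, built from modular armor meshes and a sword.
; On BeginPlay, the armor pieces follow the main Mesh through leader pose, and the sword snaps to the right-hand socket.
; Key events directly play montages for Hamstring on Q, Whirlwind on R and basic attack on left mouse, with no other ability logic in its graphs.
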(event `self.ReceiveBeginPlay`
  (bind _mesh (`self.Mesh`))
  (`SkinnedMeshComponent.SetLeaderPoseComponent` (`self.BracersAdd`) _mesh false false)
  (`SkinnedMeshComponent.SetLeaderPoseComponent` (`self.Helmet`) _mesh false false)
  (`SkinnedMeshComponent.SetLeaderPoseComponent` (`self.Shoulders`) _mesh false false)
  (`SkinnedMeshComponent.SetLeaderPoseComponent` (`self.Legs`) _mesh false false)
  (`SkinnedMeshComponent.SetLeaderPoseComponent` (`self.Hands`) _mesh false false)
  (`SkinnedMeshComponent.SetLeaderPoseComponent` (`self.HandsAdd`) _mesh false false)
  (`SkinnedMeshComponent.SetLeaderPoseComponent` (`self.Chest`) _mesh false false)
  (`SkinnedMeshComponent.SetLeaderPoseComponent` (`self.Bracers`) _mesh false false)
  (`SkinnedMeshComponent.SetLeaderPoseComponent` (`self.Boots`) _mesh false false)
  (`SkinnedMeshComponent.SetLeaderPoseComponent` (`self.Belt`) _mesh false false)
  (`SceneComponent.K2_AttachToComponent` (`self.Sword`) _mesh "hand_rSocket" "SnapToTarget" "SnapToTarget" "SnapToTarget" true))

(event `Key|Q`
  (params (Key :type "Key Structure"))
  (:`Pressed`
    (`self.PlayAnimMontage` "/Game/2HandWarrior/Animations_2HandWarrior/Abilities/AS_Hamstring_Main_Montage.AS_Hamstring_Main_Montage")))

(event `Key|R`
  (params (Key :type "Key Structure"))
  (:`Pressed`
    (`self.PlayAnimMontage` "/Game/2HandWarrior/Animations_2HandWarrior/Abilities/AM_Warrior_WhirlWind.AM_Warrior_WhirlWind")))

(event `Key|LeftMouseButton`
  (params (Key :type "Key Structure"))
  (:`Pressed`
    (`self.PlayAnimMontage` "/Game/2HandWarrior/Animations_2HandWarrior/Abilities/AM_Warrior_BasicAttacK_VersionB.AM_Warrior_BasicAttacK_VersionB")))

(fn `UserConstructionScript`)