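; BP_FireMage is the Fire Mage character Blueprint, built from modular body and armor meshes.
; On BeginPlay it sets the main Mesh as leader pose component for the ears, facial, helmet and other outfit pieces, so they follow one animated skeleton.
; Tick, overlap and the construction script contain no logic.
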(event `self.ReceiveBeginPlay`
  ;[1 1 1] SetUp Character Model
  (`SkinnedMeshComponent.SetLeaderPoseComponent` (`self.Ears`) (`self.Mesh`) false false)
  (`SkinnedMeshComponent.SetLeaderPoseComponent` (`self.Facials_01`) (`self.Mesh`) false false)
  (`SkinnedMeshComponent.SetLeaderPoseComponent` (`self.Helmet`) (`self.Mesh`) false false)
  (`SkinnedMeshComponent.SetLeaderPoseComponent` (`self.Legs`) (`self.Mesh`) false false)
  (`SkinnedMeshComponent.SetLeaderPoseComponent` (`self.Hands`) (`self.Mesh`) false false)
  (`SkinnedMeshComponent.SetLeaderPoseComponent` (`self.HandsAdd`) (`self.Mesh`) false false)
  (`SkinnedMeshComponent.SetLeaderPoseComponent` (`self.Chest`) (`self.Mesh`) false false)
  (`SkinnedMeshComponent.SetLeaderPoseComponent` (`self.Bracers`) (`self.Mesh`) false false)
  (`SkinnedMeshComponent.SetLeaderPoseComponent` (`self.Boots`) (`self.Mesh`) false false)
  (`SkinnedMeshComponent.SetLeaderPoseComponent` (`self.Belt`) (`self.Mesh`) false false)
  (`SkinnedMeshComponent.SetLeaderPoseComponent` (`self.LegsAdd`) (`self.Mesh`) false false)
  (`SkinnedMeshComponent.SetLeaderPoseComponent` (`self.BracersAdd`) (`self.Mesh`) false false)
  (`SkinnedMeshComponent.SetLeaderPoseComponent` (`self.Shoulders`) (`self.Mesh`) false false))

(fn `UserConstructionScript`)