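; AoCChampion_BP is a champion character Blueprint that carries a weapon and has a prototype hit action.
; On BeginPlay it spawns a BP_Weapon, stores it and snaps it to the mesh's "Weapon Socket".
; The A key fakes a swing by adding local pitch to the weapon root, then applying an opposite offset shortly after release.
; Both offsets also add the mesh pitch, read through an unnamed socket.
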(event `self.ReceiveBeginPlay`
  ;[1 1 1] Setup Weapon
  (bind _returnvalue (`|SpawnActorFromClass` "/Game/Blueprints/Weapon/BP_Weapon.BP_Weapon_C" (`KismetMathLibrary.Conv_VectorToTransform` (`KismetMathLibrary.MakeVector` 0.0)) "Undefined" "MultiplyWithRoot" null null))
  (set `self.NewVar` _returnvalue)
  (`self.K2_AttachToComponent` _returnvalue (`self.Mesh`) "Weapon Socket" "SnapToTarget" "SnapToTarget" "SnapToTarget" true))

(event `Key|A`
  (params (Key :type "Key Structure"))
  (bind (_returnvalue_roll _returnvalue_pitch) (`KismetMathLibrary.BreakRotator` (`SceneComponent.GetSocketRotation` (`self.Mesh`) "None")))
  (bind _rootcomponent (`Actor.RootComponent` (`self.NewVar`)))
  ;[1 1 1] Prototype Hit
  (:`Pressed`
    (`SceneComponent.K2_AddLocalRotation` _rootcomponent (`KismetMathLibrary.MakeRotator` 0.0 (+ _returnvalue_pitch 70.0)) false false))
  (:`Released`
    (`KismetSystemLibrary.Delay` 0.2)
    (`SceneComponent.K2_AddLocalRotation` _rootcomponent (`KismetMathLibrary.MakeRotator` 0.0 (- _returnvalue_pitch 70.0)) false false)))

(fn `UserConstructionScript`)